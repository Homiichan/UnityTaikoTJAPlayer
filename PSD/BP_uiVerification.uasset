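; VR verification UI attached to a usable object, letting it be checked off a task checklist and transferred to the preparation table.
; Replicated activation shows it, enables its trigger and loads its DT_TaskUI row; debug builds activate automatically.
; Task completion notifies the parent, ticks TestCheckList boxes and marks the object verified by RPC.
; On transfer, the server teleports the movable parent to a free, matching BP_EndLocation and disables its physics.
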(event `ActivateUIMulticast`
  (bind _returnvalue (`|GetDataTableRow` "/Game/_BP/DataBase/DT_TaskUI.DT_TaskUI" (`self.rowName`))
    (:`then`
      (set `self.UiStructure` _returnvalue)
      (`/Engine/EditorBlueprintResources/ActorMacros.Switch Has Authority`
        (:`Authority`
          (`self.ActivateUI`))))))

(event `self.ReceiveBeginPlay`
  (`parent.ReceiveBeginPlay`)
  (bind _assanofi_gi (cast `/Game/_BP/game/SanofiGI` (`GameplayStatics.GetGameInstance`)))
  (if (not (`/Game/VRExpansion/Vive/SanofiParentVRGameInstance.bIsDebugBuild` _assanofi_gi))
    (`KismetSystemLibrary.Delay` 2.0)
    (`SceneComponent.SetVisibility` (`self.PS`) false false)
    (`PrimitiveComponent.SetCollisionEnabled` (`self.trigger`) "NoCollision")
    (else
      (`self.ActivateUI`))))

(event `/Game/_BP/BPI_BeginPlay2Player.InterfaceBeginPlay`)

(event `TeleportActorToPreparationTable`
  (bind _returnvalue (`self.GetAttachParentActor`))
  (bind _bcanmove (`self.GetIfAttachParentActorCanBeVerified`))
  (bind _targetcheckbox (`self.TargetCheckBox`))
  (bind _rootcomponent (`Actor.RootComponent` _returnvalue))
  (bind _outactors (`GameplayStatics.GetAllActorsOfClass` "/Game/_BP/CheckMatos/BP_EndLocation.BP_EndLocation_C"))
  (for _array_element _outactors
    (if (`|EnumEquality` _targetcheckbox "NewEnumerator1")
      (bind _returnvalue_2 (`|EnumEquality` (`/Game/_BP/CheckMatos/BP_EndLocation.MatosCheck` _array_element) _targetcheckbox))
      (bind _hasmaterialssnapped (`/Game/_BP/CheckMatos/BP_EndLocation.HasMaterialsSnapped` _array_element))
      (bind _bishemoclamp (`/Game/_BP/CheckMatos/BP_EndLocation.bIsHemoClamp` _array_element))
      (`KismetSystemLibrary.PrintString` (`KismetStringLibrary.Concat_StrStr` "matos to check = " (`KismetStringLibrary.Conv_BoolToString` _returnvalue_2) "has material Snapped  " (`KismetStringLibrary.Conv_BoolToString` _hasmaterialssnapped) "canbemove   " (`KismetStringLibrary.Conv_BoolToString` _bcanmove) "parent can move   " (`KismetStringLibrary.Conv_BoolToString` _bcanmove) "is hemo clamp   " (`KismetStringLibrary.Conv_BoolToString` _bishemoclamp) "Actor = " (`KismetSystemLibrary.GetDisplayName` _returnvalue)) false false))
    (if (and _returnvalue_2 (not _hasmaterialssnapped) _bcanmove (`self.GetIfAttachParentCanBeMove`) (not _bishemoclamp))
      (set `/Game/_BP/CheckMatos/BP_EndLocation.HasMaterialsSnapped` true _array_element)
      (`SceneComponent.K2_SetWorldLocationAndRotation` _rootcomponent (`self.K2_GetActorLocation` _array_element) (`self.K2_GetActorRotation` _array_element) false true)
      (bind _asprimitive_component (cast `PrimitiveComponent` _rootcomponent)
        (:`then`
          (`PrimitiveComponent.SetSimulatePhysics` _asprimitive_component false))
        (:`CastFailed`
          _))
      (`KismetSystemLibrary.PrintString` (`KismetStringLibrary.Concat_StrStr` "I MOVE = " (`KismetSystemLibrary.GetDisplayName` _returnvalue) " endlocation" (`KismetSystemLibrary.GetDisplayName` _array_element) (`|GetEnumeratorNameAsString` _targetcheckbox)))
      (break))))

(event `ActivateUI`
  (`KismetSystemLibrary.Delay` 4.0)
  (set `self.bActivation` true)
  (`SceneComponent.SetVisibility` (`self.PS`) true false)
  (`PrimitiveComponent.SetCollisionEnabled` (`self.trigger`) "QueryAndPhysics"))

(event `SendToCheckList`
  (bind _targetcheckbox (`self.TargetCheckBox`))
  (bind _outactors (`GameplayStatics.GetAllActorsOfClass` "/Game/TestCheckList.TestCheckList_C"))
  (bind _output (`|GetArrayItem` _outactors))
  (`/Engine/EditorBlueprintResources/StandardMacros.IsValid` _output
    (:`Is Valid`
      (if (`KismetArrayLibrary.Array_Contains` (`|MakeArray` "NewEnumerator33" "NewEnumerator28" :!type "/Game/_BP/Enum/E_CheckListMateriel_D1 Enum") _targetcheckbox)
        (if (`|EnumEquality` _targetcheckbox "NewEnumerator28")
          (`/Game/TestCheckList.CheckBoxOnUI` _output _targetcheckbox true)
          (`/Game/TestCheckList.CheckBoxOnUI` _output "NewEnumerator24" true)
          (elif (`|EnumEquality` _targetcheckbox "NewEnumerator33")
            (`/Game/TestCheckList.CheckBoxOnUI` _output _targetcheckbox true)
            (`/Game/TestCheckList.CheckBoxOnUI` _output "NewEnumerator27" true)))
        (else
          (`/Game/TestCheckList.CheckBoxOnUI` _output _targetcheckbox true))))))

(event `/Game/_BP/CheckMatos/BPI_CheckMatos.OnTransfer`
  (`/Engine/EditorBlueprintResources/ActorMacros.Switch Has Authority`
    (:`Authority`
      (`self.TeleportActorToPreparationTable`))))

(event `SetIsObjectVerifiedOnUseable`
  (bind _asusable_static_mesh_base (cast `/TemplateUniVRPlugin/Game/_BP/UsableStaticMeshBase` (`self.GetParentActor`)))
  (`/TemplateUniVRPlugin/Game/_BP/UsableStaticMeshBase.SetIsVerifiedRPC` _asusable_static_mesh_base true))

(event `self.SetUIOrientation`
  (params (PawnToLookAt :type "/Game/VRExpansion/Vive/Pawn_Sanofi Object Reference"))
  (bind _scene (`self.Scene`))
  (`SceneComponent.K2_SetWorldRotation` _scene (`KismetMathLibrary.MakeRotator` (.roll (`KismetMathLibrary.FindLookAtRotation` (`SceneComponent.K2_GetComponentLocation` _scene) (`SceneComponent.K2_GetComponentLocation` (`VRBaseCharacter.VRReplicatedCamera` PawnToLookAt)))) (.pitch (`KismetMathLibrary.FindLookAtRotation` (`SceneComponent.K2_GetComponentLocation` _scene) (`SceneComponent.K2_GetComponentLocation` (`VRBaseCharacter.VRReplicatedCamera` PawnToLookAt)))) (.yaw (`KismetMathLibrary.FindLookAtRotation` (`SceneComponent.K2_GetComponentLocation` _scene) (`SceneComponent.K2_GetComponentLocation` (`VRBaseCharacter.VRReplicatedCamera` PawnToLookAt))))) false false))

(event `self.sendTaskDone`
  (params (SendValidate :type Boolean))
  (bind _returnvalue (`self.GetParentActor`))
  (`PrimitiveComponent.SetCollisionEnabled` (`self.trigger`) "NoCollision")
  (set `self.isActive` false)
  (`PrimitiveComponent.SetCollisionEnabled` (`self.valide`) "QueryOnly")
  (`PrimitiveComponent.SetCollisionEnabled` (`self.refuse`) "QueryOnly")
  (if (and (`KismetSystemLibrary.DoesImplementInterface` _returnvalue "/Game/_BP/BPI_LaserInteraction.BPI_LaserInteraction_C") (`KismetSystemLibrary.IsValid` _returnvalue))
    (message `/Game/_BP/BPI_LaserInteraction.OnValidToParent` _returnvalue null))
  (`self.SendToCheckList`)
  (`self.SetIsObjectVerifiedOnUseable`))

(fn `GetIfAttachParentActorCanBeVerified`
  (returns (bCanMove :type Boolean))
  (bind _asusable_static_mesh_base (cast `/TemplateUniVRPlugin/Game/_BP/UsableStaticMeshBase` (`self.GetAttachParentActor`))
    (:`then`
      (return true))
    (:`CastFailed`
      (return true))))

(fn `GetIfAttachParentCanBeMove`
  (returns (bCanBeMove :type Boolean))
  (locals (tmpattachparentactor :type "Actor Object Reference"))
  (bind _output_get (set `local.tmpattachparentactor` (`self.GetAttachParentActor`)))
  (bind _asusable_static_mesh_base (cast `/TemplateUniVRPlugin/Game/_BP/UsableStaticMeshBase` _output_get)
    (:`then`
      (if (`/TemplateUniVRPlugin/Game/_BP/UsableStaticMeshBase.GetCanBeMove` _asusable_static_mesh_base)
        (if (`/TemplateUniVRPlugin/Game/_BP/UsableStaticMeshBase.bIsVerified` _asusable_static_mesh_base)
          (return true)
          (else
            (`/Engine/EditorBlueprintResources/ActorMacros.Switch Has Authority`
              (:`Authority`
                (return true))
              (:`Remote`
                (return true)))))
        (else
          (return false))))
    (:`CastFailed`
      (return false))))

(fn `OnRep_bActivation`
  (`SceneComponent.SetVisibility` (`self.PS`) (`self.bActivation`) false)
  (if (`self.bActivation`)
    (`PrimitiveComponent.SetCollisionEnabled` (`self.trigger`) "QueryAndPhysics")
    (set `self.isActive` true)
    (`self.CreateDateOnServer`)
    (else
      (`PrimitiveComponent.SetCollisionEnabled` (`self.trigger`) "NoCollision")
      (set `self.isActive` false)))
  (bind _returnvalue (`|GetDataTableRow` "/Game/_BP/DataBase/DT_TaskUI.DT_TaskUI" (`self.rowName`))
    (:`then`
      (set `self.UiStructure` _returnvalue))
    (:`RowNotFound`
      _))
  (`self.CreateDateOnServer`)
  (return))

(fn `UserConstructionScript`
  (`parent.UserConstructionScript`))